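; Breakable wall actor with a DropChance function that spawns a booster pickup at its Cube's location.
; The live path almost always spawns BombRemoteBooster, because its random roll spans only values up to the threshold.
; An unconnected branch chain would choose among amount, range, speed and remote bomb boosters, rerolling at each comparison.
; The event graph and construction script are empty, and nothing here calls DropChance.
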(event EventBeginPlay)

(event Collision|EventActorBeginOverlap
  (params (OtherActor :type Actor%20Object%20Reference)))

(event EventTick
  (params (DeltaSeconds :type Float%20%28single-precision%29)))

(fn ConstructionScript)

(fn DropChance
  (if (< (Math|Random|RandomFloatinRange 0.0 3e+01) 3e+01)
    (Game|SpawnActorfromClass "/Game/Blueprints/BombRemoteBooster.BombRemoteBooster_C" (Math|Conversions|ToTransform(Vector) (Transformation|GetWorldLocation (Variables|Default|GetCube))) "Undefined" 0 0)))