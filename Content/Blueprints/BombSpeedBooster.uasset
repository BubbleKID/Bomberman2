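; BombSpeedBooster is a pickup that permanently raises the walk speed of the player who touches it.
; Overlapping its Box checks for an exact Player1 or Player2 class, then adds a fixed amount to that character's MaxWalkSpeed.
; Both branches then destroy the actor and play the Pickup sound at the Speed2 component's location with an extremely high pitch multiplier.
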(event OnComponentBeginOverlap(Box)
  (params (OverlappedComponent :type Primitive%20Component%20Object%20Reference) (OtherActor :type Actor%20Object%20Reference) (OtherComp :type Primitive%20Component%20Object%20Reference) (OtherBodyIndex :type Integer) (bFromSweep :type Boolean) (SweepResult :type Hit%20Result%20Structure%20%28by%20ref%29))
  (bind _returnvalue (Utilities|GetClass OtherActor))
  ;[1 1 1] Increase Player's  Walk Speed
  (if (== _returnvalue "/Game/Blueprints/Player1.Player1_C")
    (bind _asplayer_1 (Utilities|Casting|CastToPlayer1 OtherActor))
    (Variables|/Script/Engine.CharacterMovementComponent|SetMaxWalkSpeed (Variables|/Script/Engine.Character|GetCharacterMovement _asplayer_1) (+ (Variables|/Script/Engine.CharacterMovementComponent|GetMaxWalkSpeed (Variables|/Script/Engine.Character|GetCharacterMovement _asplayer_1)) 1e+03))
    (Actor|DestroyActor :!label _label)
    ;[1 1 1] Pick Up Sound
    (Audio|PlaySoundatLocation "/Game/Sound/pickup.pickup" (Transformation|GetWorldLocation (Variables|Default|Getspeed2)) "0, 0, 0" 1.0 1e+04)
    (elif (== _returnvalue "/Game/Blueprints/Player2.Player2_C")
      (bind _asplayer_2 (Utilities|Casting|CastToPlayer2 OtherActor))
      (Variables|/Script/Engine.CharacterMovementComponent|SetMaxWalkSpeed (Variables|/Script/Engine.Character|GetCharacterMovement _asplayer_2) (+ (Variables|/Script/Engine.CharacterMovementComponent|GetMaxWalkSpeed (Variables|/Script/Engine.Character|GetCharacterMovement _asplayer_2)) 1e+03))
      (goto _label))))

(fn ConstructionScript)