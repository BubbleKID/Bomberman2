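; BombRemoteBooster is a pickup that extends the overlapping player's bomb remote time by a fixed amount.
; Box overlap checks the actor's exact class against Player1 or Player2 and adds to the matching P1RemoteTime or P2RemoteTime on BombGameInstance.
; Both branches then destroy the booster and play the Pickup sound at the Cube's location with an extremely high pitch multiplier.
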(event OnComponentBeginOverlap(Box)
  (params (OverlappedComponent :type Primitive%20Component%20Object%20Reference) (OtherActor :type Actor%20Object%20Reference) (OtherComp :type Primitive%20Component%20Object%20Reference) (OtherBodyIndex :type Integer) (bFromSweep :type Boolean) (SweepResult :type Hit%20Result%20Structure%20%28by%20ref%29))
  (bind _returnvalue (Utilities|GetClass OtherActor))
  (if (== _returnvalue "/Game/Blueprints/Player1.Player1_C")
    (bind _asbomb_game_instance (Utilities|Casting|CastToBombGameInstance (Game|GetGameInstance)))
    (Variables|/Game/GameModes/BombGameInstance.BombGameInstance_C|SetP1_remote_time _asbomb_game_instance (+ (Variables|/Game/GameModes/BombGameInstance.BombGameInstance_C|GetP1_remote_time _asbomb_game_instance) 1e+01))
    (Actor|DestroyActor :!label _label)
    (Audio|PlaySoundatLocation "/Game/Sound/pickup.pickup" (Transformation|GetWorldLocation (Variables|Default|GetCube)) "0, 0, 0" 1.0 1e+04)
    (elif (== _returnvalue "/Game/Blueprints/Player2.Player2_C")
      (bind _asbomb_game_instance_2 (Utilities|Casting|CastToBombGameInstance (Game|GetGameInstance)))
      (Variables|/Game/GameModes/BombGameInstance.BombGameInstance_C|SetP2_remote_time _asbomb_game_instance_2 (+ (Variables|/Game/GameModes/BombGameInstance.BombGameInstance_C|GetP2_remote_time _asbomb_game_instance_2) 1e+01))
      (goto _label))))

(fn ConstructionScript)