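; Bomb amount booster pickup that raises a player's maximum bomb count.
; When an actor overlaps its Box component, an exact class check picks Player1 or Player2, casts to it and increments that class's own counter (misspelled MaxBobms on Player2).
; Both paths then destroy the booster, while other actors leave it untouched.
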(event OnComponentBeginOverlap(Box)
  (params (OverlappedComponent :type Primitive%20Component%20Object%20Reference) (OtherActor :type Actor%20Object%20Reference) (OtherComp :type Primitive%20Component%20Object%20Reference) (OtherBodyIndex :type Integer) (bFromSweep :type Boolean) (SweepResult :type Hit%20Result%20Structure%20%28by%20ref%29))
  (bind _returnvalue (Utilities|GetClass OtherActor))
  (if (== _returnvalue "/Game/Blueprints/Player1.Player1_C")
    (bind _asplayer_1 (Utilities|Casting|CastToPlayer1 OtherActor))
    (Math|Integer|IncrementInt (Variables|/Game/Blueprints/Player1.Player1_C|GetMaxBombs _asplayer_1)
      (:%20%20
        (Actor|DestroyActor :!label _label)))
    (elif (== _returnvalue "/Game/Blueprints/Player2.Player2_C")
      (bind _asplayer_2 (Utilities|Casting|CastToPlayer2 OtherActor))
      (Math|Integer|IncrementInt (Variables|/Game/Blueprints/Player2.Player2_C|GetMaxBobms _asplayer_2)
        (:%20%20
          (goto _label))))))

(fn ConstructionScript)