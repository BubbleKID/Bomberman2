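; Pickup actor that increases a player's bomb range in a two-player bomb game.
; On box overlap it checks whether the other actor is exactly Player1 or Player2 and adds a fixed amount to that player's bomb range on BombGameInstance.
; It then destroys itself; only the Player1 branch prints the new range to screen.
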(event OnComponentBeginOverlap(Box)
  (params (OverlappedComponent :type Primitive%20Component%20Object%20Reference) (OtherActor :type Actor%20Object%20Reference) (OtherComp :type Primitive%20Component%20Object%20Reference) (OtherBodyIndex :type Integer) (bFromSweep :type Boolean) (SweepResult :type Hit%20Result%20Structure%20%28by%20ref%29))
  (bind _returnvalue (Utilities|GetClass OtherActor))
  (bind _returnvalue_2 (Game|GetGameInstance))
  (if (== _returnvalue "/Game/Blueprints/Player1.Player1_C")
    (bind _asbomb_game_instance (Utilities|Casting|CastToBombGameInstance _returnvalue_2))
    (bind _output_get (Variables|/Game/GameModes/BombGameInstance.BombGameInstance_C|SetPlayer1BombRange _asbomb_game_instance (+ (Variables|/Game/GameModes/BombGameInstance.BombGameInstance_C|GetPlayer1BombRange _asbomb_game_instance) 3e+01)))
    (Development|PrintString (Utilities|String|ToString(Float) _output_get))
    (Actor|DestroyActor :!label _label)
    (elif (== _returnvalue "/Game/Blueprints/Player2.Player2_C")
      (bind _asbomb_game_instance_2 (Utilities|Casting|CastToBombGameInstance _returnvalue_2))
      (Variables|/Game/GameModes/BombGameInstance.BombGameInstance_C|SetPlayer2BombRange _asbomb_game_instance_2 (+ (Variables|/Game/GameModes/BombGameInstance.BombGameInstance_C|GetPlayer2BombRange _asbomb_game_instance_2) 3e+01))
      (goto _label))))

(fn ConstructionScript)