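; Player 2's Bomberman-style bomb, which explodes after an animated material-and-light fuse or when the Boom2 event fires.
; BeginPlay sizes two crossed blast boxes from the GameInstance range; their overlaps destroy players, breakable walls and boosters.
; Any player death flags Player 1's win, though the event path writes Player2Score.
; Detonation spawns cross-shaped emitters and updates P2BombArray; the sphere blocks pawns once its instigator steps off.
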(event OnComponentEndOverlap(Sphere)
  (params (OverlappedComponent :type Primitive%20Component%20Object%20Reference) (OtherActor :type Actor%20Object%20Reference) (OtherComp :type Primitive%20Component%20Object%20Reference) (OtherBodyIndex :type Integer))
  (bind _asplayer_2 (Utilities|Casting|CastToPlayer2 OtherActor))
  (if (== _asplayer_2 (Game|GetInstigator))
    (Collision|SetCollisionResponsetoChannel (Variables|Default|GetSphere) "ECC_Pawn" "ECR_Block")))

(event Custom|boom2_Event
  (bind _asbomb_game_instance (Utilities|Casting|CastToBombGameInstance (Game|GetGameInstance)))
  ;[1 1 1] Explosion sound
  (Audio|PlaySoundatLocation "/Game/StarterContent/Audio/Explosion01.Explosion01" (Transformation|GetWorldLocation (Variables|Default|GetSphere)))
  (bind _outactors (Actor|GetAllActorsOfClass "/Game/Blueprints/Player2.Player2_C"))
  (for _array_element _outactors
    (Math|Integer|DecrementInt (Variables|/Game/Blueprints/Player2.Player2_C|GetCurrentBobms _array_element)))
  ;[1 1 1] merge 2 collisions
  (bind _output_get (Variables|Default|Setbomb_opverlapping (Collision|GetOverlappingActors (Variables|Default|GetBlastBoxY) 0 :!class /Script/Engine.PrimitiveComponent)))
  (for _array_element_2 (Collision|GetOverlappingActors (Variables|Default|GetBlastBoxX) 0 :!class /Script/Engine.PrimitiveComponent)
    (Utilities|Array|Add _output_get _array_element_2))
  (for _array_element_3 (Variables|Default|Getbomb_opverlapping)
    (if (or (== (Utilities|GetClass _array_element_3) "/Game/Blueprints/Player1.Player1_C") (== (Utilities|GetClass _array_element_3) "/Game/Blueprints/Player2.Player2_C"))
      (Actor|DestroyActor _array_element_3)
      ;[1 1 1] add players' score
      (bind _asbomb_game_instance_2 (Utilities|Casting|CastToBombGameInstance (Game|GetGameInstance)))
      (Variables|/Game/GameModes/BombGameInstance.BombGameInstance_C|SetPlayer1Win _asbomb_game_instance_2 true)
      (bind _result (Math|Integer|IncrementInt (Variables|/Game/GameModes/BombGameInstance.BombGameInstance_C|GetPlayer1Score _asbomb_game_instance_2))
        (:%20%20
          (Variables|/Game/GameModes/BombGameInstance.BombGameInstance_C|Setplayer2Score _asbomb_game_instance_2 _result)
          (bind _returnvalue (UserInterface|CreateWidget "/Game/UI/UI_Win.UI_Win_C" (Game|GetPlayerController 0)))
          (UserInterface|Viewport|AddtoViewport _returnvalue 0)))
      (elif (== (Utilities|GetClass _array_element_3) "/Game/Blueprints/Breakable_wall.Breakable_wall_C")
        (bind _asbreakable_wall (Utilities|Casting|CastToBreakable_wall _array_element_3))
        (Default|DropChance _asbreakable_wall)
        (Actor|DestroyActor _array_element_3)
        (elif (Math|Boolean|ORBoolean (== (Utilities|GetClass _array_element_3) "/Game/Blueprints/BombAmountBooster.BombAmountBooster_C") (== (Utilities|GetClass _array_element_3) "/Game/Blueprints/BombRangeBooster.BombRangeBooster_C") (== (Utilities|GetClass _array_element_3) "/Game/Blueprints/BombRemoteBooster.BombRemoteBooster_C") (== (Utilities|GetClass _array_element_3) "/Game/Blueprints/BombSpeedBooster.BombSpeedBooster_C"))
          (Actor|DestroyActor _array_element_3)
          (elif (or (== (Utilities|GetClass _array_element_3) "/Game/Blueprints/Bomb1.Bomb1_C") (== (Utilities|GetClass _array_element_3) "Bomb2_C"))
            _)))))
  ;[1 1 1] bomb destroy
  (CallFunction|ShowBlast2)
  (Actor|DestroyActor (Utilities|Array|Get(acopy) (Variables|/Game/GameModes/BombGameInstance.BombGameInstance_C|GetP2_bomb_array _asbomb_game_instance)))
  (bind _asbomb_game_instance_3 (Utilities|Casting|CastToBombGameInstance (Game|GetGameInstance)))
  (bind _output_get_2 (Variables|/Game/GameModes/BombGameInstance.BombGameInstance_C|SetP2_bomb_array _asbomb_game_instance_3 (Variables|/Game/GameModes/BombGameInstance.BombGameInstance_C|GetP2_bomb_array _asbomb_game_instance_3)))
  (Utilities|Array|RemoveIndex _output_get_2)
  (for _array_element_4 (Variables|/Game/GameModes/BombGameInstance.BombGameInstance_C|GetP2_bomb_array _asbomb_game_instance_3)
    _))

(event EventBeginPlay
  (bind _pointlight (Variables|Default|GetPointLight))
  (EventDispatchers|BindEventtoBoom2 (delegate Custom|boom2_Event))
  ;[1 1 1] set bomb collision
  (bind _asbomb_game_instance (Utilities|Casting|CastToBombGameInstance (Game|GetGameInstance)))
  (Variables|Default|SetGame%20Instance _asbomb_game_instance)
  (Components|Box|SetBoxExtent (Variables|Default|GetBlastBoxX) (Math|Vector|MakeVector 0.0 (Variables|/Game/GameModes/BombGameInstance.BombGameInstance_C|GetPlayer2BombRange (Variables|Default|GetGame%20Instance)) 0.0) true)
  (Components|Box|SetBoxExtent (Variables|Default|GetBlastBoxY) (Math|Vector|MakeVector (Variables|/Game/GameModes/BombGameInstance.BombGameInstance_C|GetPlayer2BombRange (Variables|Default|GetGame%20Instance)) 0.0 0.0) true)
  ;[1 1 1] bomb animation
  (Rendering|Material|SetMaterial (Variables|Default|GetSphere) 0 "/Game/Materials/MAT_bomb1.MAT_bomb1")
  (Utilities|FlowControl|Delay 0.5)
  (Rendering|Components|Light|SetIntensity _pointlight 2e+03)
  (Rendering|Material|SetMaterial (Variables|Default|GetSphere) 0 "/Game/Materials/MAT_bomb2.MAT_bomb2")
  (Utilities|FlowControl|Delay 0.5)
  (Rendering|Components|Light|SetIntensity _pointlight 3e+03)
  (Rendering|Material|SetMaterial (Variables|Default|GetSphere) 0 "/Game/Materials/MAT_bomb3.MAT_bomb3")
  (Utilities|FlowControl|Delay 0.5)
  (Rendering|Components|Light|SetIntensity _pointlight 4e+03)
  (Rendering|Material|SetMaterial (Variables|Default|GetSphere) 0 "/Game/Materials/MAT_bomb4.MAT_bomb4")
  (Utilities|FlowControl|Delay 0.5)
  (Rendering|Components|Light|SetIntensity _pointlight 5e+03)
  (Utilities|FlowControl|Delay 0.5)
  ;[1 1 1] Explosion sound
  (Audio|PlaySoundatLocation "/Game/StarterContent/Audio/Explosion01.Explosion01" (Transformation|GetWorldLocation (Variables|Default|GetSphere)))
  (bind _outactors (Actor|GetAllActorsOfClass "/Game/Blueprints/Player2.Player2_C"))
  (for _array_element _outactors
    (Math|Integer|DecrementInt (Variables|/Game/Blueprints/Player2.Player2_C|GetCurrentBobms _array_element)))
  (bind _output_get (Variables|Default|Setbomb_opverlapping (Collision|GetOverlappingActors (Variables|Default|GetBlastBoxY) 0 :!class /Script/Engine.PrimitiveComponent)))
  (for _array_element_2 (Collision|GetOverlappingActors (Variables|Default|GetBlastBoxX) 0 :!class /Script/Engine.PrimitiveComponent)
    (Utilities|Array|Add _output_get _array_element_2))
  (for _array_element_3 (Variables|Default|Getbomb_opverlapping)
    (if (or (== (Utilities|GetClass _array_element_3) "/Game/Blueprints/Player1.Player1_C") (== (Utilities|GetClass _array_element_3) "/Game/Blueprints/Player2.Player2_C"))
      (Actor|DestroyActor _array_element_3)
      ;[1 1 1] add players' score
      (bind _asbomb_game_instance_2 (Utilities|Casting|CastToBombGameInstance (Game|GetGameInstance)))
      (Variables|/Game/GameModes/BombGameInstance.BombGameInstance_C|SetPlayer1Win _asbomb_game_instance_2 true)
      (bind _result (Math|Integer|IncrementInt (Variables|/Game/GameModes/BombGameInstance.BombGameInstance_C|GetPlayer1Score _asbomb_game_instance_2))
        (:%20%20
          (Variables|/Game/GameModes/BombGameInstance.BombGameInstance_C|SetPlayer1Score _asbomb_game_instance_2 _result)
          (bind _returnvalue (UserInterface|CreateWidget "/Game/UI/UI_Win.UI_Win_C" (Game|GetPlayerController 0)))
          (UserInterface|Viewport|AddtoViewport _returnvalue 0)))
      (elif (== (Utilities|GetClass _array_element_3) "/Game/Blueprints/Breakable_wall.Breakable_wall_C")
        (bind _asbreakable_wall (Utilities|Casting|CastToBreakable_wall _array_element_3))
        (Default|DropChance _asbreakable_wall)
        (Actor|DestroyActor _array_element_3)
        (elif (Math|Boolean|ORBoolean (== (Utilities|GetClass _array_element_3) "/Game/Blueprints/BombAmountBooster.BombAmountBooster_C") (== (Utilities|GetClass _array_element_3) "/Game/Blueprints/BombRangeBooster.BombRangeBooster_C") (== (Utilities|GetClass _array_element_3) "/Game/Blueprints/BombRemoteBooster.BombRemoteBooster_C") (== (Utilities|GetClass _array_element_3) "/Game/Blueprints/BombSpeedBooster.BombSpeedBooster_C"))
          (Actor|DestroyActor _array_element_3)
          (elif (or (== (Utilities|GetClass _array_element_3) "/Game/Blueprints/Bomb1.Bomb1_C") (== (Utilities|GetClass _array_element_3) "Bomb2_C"))
            _)))))
  ;[1 1 1] bomb destroy
  (CallFunction|ShowBlast2)
  (Actor|DestroyActor)
  (bind _asbomb_game_instance_3 (Utilities|Casting|CastToBombGameInstance (Game|GetGameInstance)))
  (bind _output_get_2 (Variables|/Game/GameModes/BombGameInstance.BombGameInstance_C|SetP2_bomb_array _asbomb_game_instance_3 (Variables|/Game/GameModes/BombGameInstance.BombGameInstance_C|GetP2_bomb_array _asbomb_game_instance_3)))
  (Utilities|Array|RemoveIndex _output_get_2)
  (for _array_element_4 (Variables|/Game/GameModes/BombGameInstance.BombGameInstance_C|GetP2_bomb_array _asbomb_game_instance_3)
    _))

(fn ConstructionScript)

(fn ShowBlast2
  (bind _sphere1 (Variables|Default|GetSphere1))
  (bind _sphere (Variables|Default|GetSphere))
  (bind _sphere_2 (Variables|Default|GetSphere))
  (bind _returnvalue (Transformation|GetWorldLocation _sphere_2))
  (bind _returnvalue_2 (Transformation|GetWorldLocation _sphere))
  (bind _sphereradius (Variables|/Script/Engine.SphereComponent|GetSphereRadius _sphere1))
  (bind (_x _y _z) (Math|Vector|BreakVector _returnvalue_2))
  (bind (_x_2 _y_2 _z_2) (Math|Vector|BreakVector _returnvalue))
  (bind _returnvalue_3 (/ _sphereradius 3e+01))
  (bind _returnvalue_4 (Math|Float|Truncate _returnvalue_3))
  (for _index (range (* _returnvalue_4 -1) _returnvalue_4)
    (Effects|SpawnEmitteratLocation "/Game/StarterContent/Particles/P_Explosion.P_Explosion" (Math|Vector|MakeVector (+ (* (Math|Conversions|ToFloat(Integer) _index) 3e+01) _x_2) _y_2 _z_2))
    (Effects|SpawnEmitteratLocation "/Game/StarterContent/Particles/P_Explosion.P_Explosion" (Math|Vector|MakeVector _x (+ (* (Math|Conversions|ToFloat(Integer) _index) 3e+01) _y) _z))))