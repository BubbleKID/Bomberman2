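; Player 1 character for a bomb-laying game, moved by applying input-axis forces to a physics cube each tick.
; Space spawns a Bomb1 above the cube until the bomb cap is reached, registering it in BombGameInstance's P1 array.
; F detonates every Bomb1 while the game instance's P1RemoteTime is positive.
; Tick counts down a separate local RemoteTime1, which the detonation check does not read.
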(event EventTick
  (params (DeltaSeconds :type Float%20%28single-precision%29))
  (bind _movementspeed (Variables|Default|GetMovementSpeed))
  ;[1 1 1] Movement
  (Physics|AddForce (Variables|Default|GetCube) (Math|Vector|MakeVector (* (Input|AxisValues|Getforward1) _movementspeed) (* (Input|AxisValues|Getright1) _movementspeed) 0.0) "None" false)
  (if (> (Variables|Default|GetRemoteTime1) 0.0)
    (Variables|Default|SetRemoteTime1 (- (Variables|Default|GetRemoteTime1) DeltaSeconds))))

(event Input|KeyboardEvents|SpaceBar
  (params (Key :type Key%20Structure))
  ;[1 1 1] SpawnBombs
  (:Pressed
    (CallFunction|SpawnBombs)))

(event Input|KeyboardEvents|F
  (params (Key :type Key%20Structure))
  ;[1 1 1] activate bomb
  (:Pressed
    (CallFunction|RemoteBomb)))

(fn ConstructionScript)

(fn SpawnBombs
  (bind _cube (Variables|Default|GetCube))
  (bind _returnvalue (Transformation|GetWorldLocation _cube))
  (bind (_x _y _z) (Math|Vector|BreakVector _returnvalue))
  (if (!= (Variables|Default|GetCurrentBombs) (Variables|Default|GetMaxBombs))
    (bind _returnvalue_2 (Game|SpawnActorfromClass "/Game/Blueprints/Bomb1.Bomb1_C" (Math|Conversions|ToTransform(Vector) (Math|Vector|MakeVector _x _y (+ _z 2e+02))) "Undefined" 0 0))
    (Math|Integer|IncrementInt (Variables|Default|GetCurrentBombs)
      (:%20%20
        (bind _asbomb_game_instance (Utilities|Casting|CastToBombGameInstance (Game|GetGameInstance)))
        (Utilities|Array|Add (Variables|/Game/GameModes/BombGameInstance.BombGameInstance_C|GetP1_bomb_array _asbomb_game_instance) _returnvalue_2)))))

(fn RemoteBomb
  (bind _asbomb_game_instance (Utilities|Casting|CastToBombGameInstance (Game|GetGameInstance)))
  (if (> (Variables|/Game/GameModes/BombGameInstance.BombGameInstance_C|GetP1_remote_time _asbomb_game_instance) 0.0)
    (bind _outactors (Actor|GetAllActorsOfClass "/Game/Blueprints/Bomb1.Bomb1_C"))
    (for _array_element _outactors
      (bind _asbomb_1 (Utilities|Casting|CastToBomb1 _array_element))
      (Default|BoomEvent _asbomb_1))))