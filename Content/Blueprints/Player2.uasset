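; Player 2 pawn logic for a bomb game, covering bomb placement and remote detonation.
; SpawnBomb2 spawns a Bomb2 just above the mesh's location unless the count equals the maximum, then increments the count and records the bomb in BombGameInstance's P2 array.
; Remotebomb2 checks that the game instance's P2 remote time is positive, then triggers every Bomb2 found through GetAllActorsOfClass, not the stored array.
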(fn ConstructionScript)

(fn SpawnBomb2
  (bind _mesh (Variables|Character|GetMesh))
  (bind _returnvalue (Transformation|GetWorldLocation _mesh))
  (bind (_x _y _z) (Math|Vector|BreakVector _returnvalue))
  (if (!= (Variables|Default|GetMaxBombs) (Variables|Default|GetCurrentBobms))
    (bind _returnvalue_2 (Game|SpawnActorfromClass "/Game/Blueprints/Bomb2.Bomb2_C" (Math|Conversions|ToTransform(Vector) (Math|Vector|MakeVector _x _y (+ _z 7e+01))) "Undefined" 0 0))
    (Math|Integer|IncrementInt (Variables|Default|GetCurrentBobms)
      (:%20%20
        (bind _asbomb_game_instance (Utilities|Casting|CastToBombGameInstance (Game|GetGameInstance)))
        (Utilities|Array|Add (Variables|/Game/GameModes/BombGameInstance.BombGameInstance_C|GetP2_bomb_array _asbomb_game_instance) _returnvalue_2)))))

(fn Remotebomb2
  (bind _asbomb_game_instance (Utilities|Casting|CastToBombGameInstance (Game|GetGameInstance)))
  (if (> (Variables|/Game/GameModes/BombGameInstance.BombGameInstance_C|GetP2_remote_time _asbomb_game_instance) 0.0)
    (bind _outactors (Actor|GetAllActorsOfClass "/Game/Blueprints/Bomb2.Bomb2_C"))
    (for _array_element _outactors
      (bind _asbomb_2 (Utilities|Casting|CastToBomb2 _array_element))
      (Default|CallBoom2 _asbomb_2))))